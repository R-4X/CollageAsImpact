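; Player character for the Chronologie game mode that lets the player pick up BP_ObjectChronologie actors with the mouse and drag them.
; When IA_DragAndDrop starts, a Visibility trace from the deprojected cursor stores the hit object and disables its collision.
; While the input triggers, the same trace moves that object to the hit location.
; StopDrag only clears the held reference; nothing here calls it or restores collision.
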(event Input|EnhancedActionEvents|EnhancedInputActionIA_DragAndDrop
  (params (ActionValue :type Boolean) (ElapsedSeconds :type Float%20%28double-precision%29) (TriggeredSeconds :type Float%20%28double-precision%29) (InputAction :type Input%20Action%20Object%20Reference :default "/Game/CollageAsImpact/ChronologieGamemode/Control/Action/IA_DragAndDrop.IA_DragAndDrop"))
  (:Triggered
    (CallFunction|Drag))
  (:Started
    (CallFunction|TakeObject)))

(fn ConstructionScript)

(fn TakeObject
  (bind (_location _direction) (CallFunction|GetMouseLocation))
  (bind _outhit (Collision|LineTraceByChannel _location _direction "TraceTypeQuery1" false 0 "None"))
  (bind _output_get (LocalVariables|SetHitActor (.HitActor (Collision|BreakHitResult _outhit))))
  (bind _asbp_object_chronologie (Utilities|Casting|CastToBP_ObjectChronologie _output_get))
  (bind _output_get_2 (Variables|Default|Set_whatITake _asbp_object_chronologie))
  (Collision|SetActorEnableCollision _output_get_2 false)
  (return))

(fn GetMouseLocation
  (bind _returnvalue (Game|GetPlayerController 0))
  (bind (_worldlocation _worlddirection) (Game|Player|ConvertMouseLocationToWorldSpace _returnvalue))
  (return _worldlocation (+ _worlddirection (* _worlddirection (Variables|Default|Get_range)))))

(fn Drag
  (bind (_location _direction) (CallFunction|GetMouseLocation))
  (Utilities|IsValid (Variables|Default|Get_whatITake)
    (:Is%20Valid
      (bind _outhit (Collision|LineTraceByChannel _location _direction "TraceTypeQuery1" false 0 "None"))
      (Transformation|SetActorLocation (Variables|Default|Get_whatITake) (Math|Vector|MakeVector (.X (Math|Vector|BreakVector (.Location (Collision|BreakHitResult _outhit)))) (.Y (Math|Vector|BreakVector (.Location (Collision|BreakHitResult _outhit)))) (.Z (Math|Vector|BreakVector (.Location (Collision|BreakHitResult _outhit))))) false false))))

(fn StopDrag
  (Variables|Default|Set_whatITake 0))