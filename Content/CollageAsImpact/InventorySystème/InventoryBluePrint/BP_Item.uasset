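; BP_Item is a physics-simulated world pickup whose static mesh comes from its Item data in the construction script.
; When the top-down character overlaps its sphere and CanTake is set, it calls TakeItem on that character's inventory component, passing a short vertical segment from the mesh location.
; Interact tells a referenced Door to show its key pickup message, then destroys the item, while LookAt returns empty text.
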(event OnComponentBeginOverlap(Sphere)
  (params (OverlappedComponent :type Primitive%20Component%20Object%20Reference) (OtherActor :type Actor%20Object%20Reference) (OtherComp :type Primitive%20Component%20Object%20Reference) (OtherBodyIndex :type Integer) (bFromSweep :type Boolean) (SweepResult :type Hit%20Result%20Structure%20%28by%20ref%29))
  (bind _staticmesh (Variables|Default|GetStaticMesh))
  (bind _returnvalue (Transformation|GetWorldLocation _staticmesh))
  (bind _asbp_top_down_character (Utilities|Casting|CastToBP_TopDownCharacter OtherActor))
  (if (Variables|Default|Get_canTake?)
    (Default|TakeItem (Variables|/Game/TopDown/Blueprints/BP_TopDownCharacter.BP_TopDownCharacter_C|GetBP_InventoryComponent _asbp_top_down_character) _returnvalue (+ _returnvalue "0.000000,0.000000,10.000000"))))

(event EventInteract
  (Class|BPIKey|PickUpKey(Message) (Variables|Default|GetDoor))
  (Actor|DestroyActor))

(fn ConstructionScript
  (bind _staticmesh (Variables|Default|GetStaticMesh))
  (Components|StaticMesh|SetStaticMesh _staticmesh (.Mesh (Utilities|Struct|BreakS_ItemStructure (Variables|Default|Get_item))))
  (Physics|SetSimulatePhysics _staticmesh true))

(fn Lookat
  (return ""))