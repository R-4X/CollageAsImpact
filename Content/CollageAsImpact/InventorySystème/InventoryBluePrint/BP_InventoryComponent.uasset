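; Inventory component that holds an eight-slot item array and shows it in a WBP_Inventory widget created on BeginPlay.
; TakeItem sphere-traces for a BP_Item, then walks the slots, incrementing a matching stackable entry within a 64 limit or filling an empty slot.
; A successful pickup reloads the widget, calls GrabKey on BP_TopDownCharacter and destroys the item, whose validity check stops further inserts.
; LookAt is an empty stub.
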(event Custom|TakeItem
  (params (Start :type Vector) (End :type Vector))
  ;[0.15 0.15 0.15 0.5] When take item in box collide put it in inventory and show sprite
  ;;[0.15 0.06797 0.06797 0.5] Create box and detecte item
  (bind _outhit (Collision|SphereTraceByChannel Start End 1.2e+02 "TraceTypeQuery1" false 0 "ForDuration"))
  (bind _asbp_item (Utilities|Casting|CastToBP_Item (.HitActor (Collision|BreakHitResult _outhit))))
  (for (_array_element _array_index) (Variables|Default|GetItem)
    (Utilities|IsValid _asbp_item
      (:Is%20Valid
        (if (Math|Boolean|ANDBoolean (Utilities|Enum|Equal(Enum) (.Name (Utilities|Struct|BreakS_ItemStructure _array_element)) (.Name (Utilities|Struct|BreakS_ItemStructure (Variables|/Game/CollageAsImpact/InventorySystème/InventoryBluePrint/BP_Item.BP_Item_C|Get_item _asbp_item)))) (.Stackable (Utilities|Struct|BreakS_ItemStructure (Variables|/Game/CollageAsImpact/InventorySystème/InventoryBluePrint/BP_Item.BP_Item_C|Get_item _asbp_item))) (<= (+ (.Quantity (Utilities|Struct|BreakS_ItemStructure _array_element)) (.Quantity (Utilities|Struct|BreakS_ItemStructure (Variables|/Game/CollageAsImpact/InventorySystème/InventoryBluePrint/BP_Item.BP_Item_C|Get_item _asbp_item)))) 64))
          (Utilities|Array|SetArrayElem (Variables|Default|GetItem) _array_index (Utilities|Struct|MakeS_ItemStructure (.name (Variables|/Game/CollageAsImpact/InventorySystème/InventoryBluePrint/BP_Item.BP_Item_C|Get_item _asbp_item)) (.stackable (Variables|/Game/CollageAsImpact/InventorySystème/InventoryBluePrint/BP_Item.BP_Item_C|Get_item _asbp_item)) (+ (.Quantity (Utilities|Struct|BreakS_ItemStructure _array_element)) 1) (.thumnail (Variables|/Game/CollageAsImpact/InventorySystème/InventoryBluePrint/BP_Item.BP_Item_C|Get_item _asbp_item)) (.mesh (Variables|/Game/CollageAsImpact/InventorySystème/InventoryBluePrint/BP_Item.BP_Item_C|Get_item _asbp_item))))
          (Default|LoadInventory (Variables|Default|GetInventoryWidget) self :!label _label)
          (bind _returnvalue (Actor|GetActorOfClass "/Game/TopDown/Blueprints/BP_TopDownCharacter.BP_TopDownCharacter_C"))
          (Default|GrabKey _returnvalue)
          (Actor|DestroyActor _asbp_item)
          (elif (== (.Quantity (Utilities|Struct|BreakS_ItemStructure _array_element)) 0)
            (Utilities|Array|SetArrayElem (Variables|Default|GetItem) _array_index (Variables|/Game/CollageAsImpact/InventorySystème/InventoryBluePrint/BP_Item.BP_Item_C|Get_item _asbp_item))
            (goto _label)))))))

(event EventBeginPlay
  ;[0.15 0.15 0.15 0.5] Set inventory and number of item case
  (bind _returnvalue (UserInterface|CreateWidget "/Game/CollageAsImpact/InventorySystème/InventoryWidget/WBP_Inventory.WBP_Inventory_C"))
  (Variables|Default|SetInventoryWidget _returnvalue)
  (Utilities|Array|Resize (Variables|Default|GetItem) 8)
  (Default|LoadInventory (Variables|Default|GetInventoryWidget) self)
  ;[0.15 0.15 0.15 0.5] Show Inventry widget + set input mode
  (UserInterface|Viewport|AddtoViewport (Variables|Default|GetInventoryWidget) 0))

(fn Lookat
  (return ""))