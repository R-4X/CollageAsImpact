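; BP_MAnagerDTL is a trigger actor that drives the exfiltration checklist widget, WBP_ExfiltrationTDL.
; It creates and displays the widget on BeginPlay.
; When BP_TopDownCharacter enters its Box, it ticks CheckBox2, plays a page-turn sound and removes the widget after a short delay.
; Leaving the Box unticks the checkbox but neither cancels the removal nor restores the widget; both overlaps print debug text.
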(event OnComponentBeginOverlap(Box)
  (params (OverlappedComponent :type Primitive%20Component%20Object%20Reference) (OtherActor :type Actor%20Object%20Reference) (OtherComp :type Primitive%20Component%20Object%20Reference) (OtherBodyIndex :type Integer) (bFromSweep :type Boolean) (SweepResult :type Hit%20Result%20Structure%20%28by%20ref%29))
  (Utilities|Casting|CastToBP_TopDownCharacter OtherActor)
  (Development|PrintString "Hello")
  (Class|CheckBox|SetIsChecked (Variables|/Game/CollageAsImpact/ContentImage/WBP/ToDoList/WBP_ExfiltrationTDL.WBP_ExfiltrationTDL_C|GetCheckBox_2 (Variables|Default|GetWBP_TDL)) true)
  (Audio|PlaySound2D "/Game/CollageAsImpact/Sound/Book/PageJournalTurn.PageJournalTurn" 1.0 1.0 0.0 0 0)
  (Utilities|FlowControl|Delay 1.5)
  (Widget|RemovefromParent (stale EventBeginPlay _output_get)))

(event OnComponentEndOverlap(Box)
  (params (OverlappedComponent :type Primitive%20Component%20Object%20Reference) (OtherActor :type Actor%20Object%20Reference) (OtherComp :type Primitive%20Component%20Object%20Reference) (OtherBodyIndex :type Integer))
  (Utilities|Casting|CastToBP_TopDownCharacter OtherActor)
  (Development|PrintString "Hello")
  (Class|CheckBox|SetIsChecked (Variables|/Game/CollageAsImpact/ContentImage/WBP/ToDoList/WBP_ExfiltrationTDL.WBP_ExfiltrationTDL_C|GetCheckBox_2 (Variables|Default|GetWBP_TDL)) false))

(event EventBeginPlay
  (bind _returnvalue (UserInterface|CreateWidget "/Game/CollageAsImpact/ContentImage/WBP/ToDoList/WBP_ExfiltrationTDL.WBP_ExfiltrationTDL_C"))
  (UserInterface|Viewport|AddtoViewport _returnvalue 0)
  (bind _output_get (Variables|Default|SetWBP_TDL _returnvalue)))

(event Collision|EventActorBeginOverlap
  (params (OtherActor :type Actor%20Object%20Reference)))

(event EventTick
  (params (DeltaSeconds :type Float%20%28single-precision%29)))

(fn ConstructionScript)