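; BP_ManagerLight is a manager that creates a neon flicker effect on a set of referenced point lights.
; On BeginPlay it starts a fast looping timer that calls LightIntensity.
; Each tick of that timer sets random intensities on two main lights and a dimmer range on five PointLightman lights.
; The same event also plays the Neonflickering 2D sound, so the sound retriggers on every timer tick.
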(event Custom|LightIntensity
  (Rendering|Components|Light|SetIntensity (Variables|/Script/Engine.PointLight|GetPointLightComponent (Variables|Default|GetPointLight)) (Math|Random|RandomFloatinRange 8.0 1e+01))
  (Rendering|Components|Light|SetIntensity (Variables|/Script/Engine.Light|GetLightComponent (Variables|Default|GetPointLight2)) (Math|Random|RandomFloatinRange 8.0 15.0))
  (Rendering|Components|Light|SetIntensity (Variables|/Script/Engine.Light|GetLightComponent (Variables|Default|GetPointLightman1)) (Math|Random|RandomFloatinRange 1.0 5.0))
  (Audio|PlaySound2D "/Game/CollageAsImpact/Sound/Environnement/Bp_RailShooter/neonflickering.neonflickering" 0.5 1.0 0.0 0 0))

(event EventBeginPlay
  (Utilities|Time|SetTimerbyEvent (delegate Custom|LightIntensity) 0.05 true))

(fn ConstructionScript)