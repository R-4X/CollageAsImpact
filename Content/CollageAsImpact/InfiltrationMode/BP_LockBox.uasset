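; BP_LockBox is an infiltration-mode lock that completes when a BP_Item with a matching ID overlaps its Box trigger.
; An optional BoxNeed reference chains it behind another object, so items only count once that object is Complete.
; On a match it destroys the item, sets Complete, then unhides its Cube and enables the collision that BeginPlay turned off.
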(event OnComponentBeginOverlap(Box)
  (params (OverlappedComponent :type Primitive%20Component%20Object%20Reference) (OtherActor :type Actor%20Object%20Reference) (OtherComp :type Primitive%20Component%20Object%20Reference) (OtherBodyIndex :type Integer) (bFromSweep :type Boolean) (SweepResult :type Hit%20Result%20Structure%20%28by%20ref%29))
  (bind _cube (Variables|Default|GetCube))
  (bind _asbp_item (Utilities|Casting|CastToBP_Item OtherActor))
  (Utilities|IsValid (Variables|Default|GetBoxNeed)
    (:Is%20Valid
      (if (Variables|BP_LockBox_C|GetComplete (Variables|Default|GetBoxNeed))
        (if (Utilities|Enum|Equal(Enum) (.ID (Utilities|Struct|BreakS_ItemStructure (Variables|/Game/CollageAsImpact/InventorySystème/InventoryBluePrint/BP_Item.BP_Item_C|Get_item _asbp_item))) (Variables|Default|GetID)) :!label _label
          (Actor|DestroyActor _asbp_item)
          (Variables|Default|SetComplete true)
          (Development|SetHiddeninGame _cube false false)
          (Collision|SetCollisionEnabled _cube "QueryAndPhysics"))))
    (:Is%20Not%20Valid
      (goto _label))))

(event EventBeginPlay
  (Collision|SetCollisionEnabled (Variables|Default|GetCube) "NoCollision"))

(fn ConstructionScript)