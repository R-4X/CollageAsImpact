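; Pursuing AI character for Infiltration Mode that chases the player and speeds up the farther away it is.
; On BeginPlay it writes the player character to the Blackboard and starts a looping timer.
; The timer sets walk speed from 2D distance to the player, clamped between minimum and maximum speeds.
; Pawn sensing sets the Blackboard "See" flag when a pawn is spotted, and nothing here clears it.
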(event OnSeePawn(PawnSensing)
  (params (Pawn :type Pawn%20Object%20Reference))
  (AI|Components|Blackboard|SetValueasBool (AI|GetBlackboard (AI|GetAIController self)) (Utilities|Name|MakeLiteralName "See") true))

(event Custom|SetSpeed
  (bind _returnvalue (Transformation|GetActorLocation))
  (bind _returnvalue_2 (Game|GetPlayerCharacter 0))
  (bind _returnvalue_3 (Transformation|GetActorLocation _returnvalue_2))
  (Variables|/Script/Engine.CharacterMovementComponent|SetMaxWalkSpeed (Variables|Character|GetCharacterMovement) (Math|Float|Clamp(Float) (* (Math|Vector|Distance2D(Vector) (Math|Vector2D|MakeVector2D (.x _returnvalue) (.y _returnvalue)) (Math|Vector2D|MakeVector2D (.x _returnvalue_3) (.y _returnvalue_3))) 1.5) (Variables|Default|GetMinWalkSpeed) (Variables|Default|GetMaxWalkSpeed))))

(event EventBeginPlay
  (AI|Components|Blackboard|SetValueasObject (AI|GetBlackboard (AI|GetAIController self)) (Utilities|Name|MakeLiteralName "Player") (Game|GetPlayerCharacter 0))
  (Utilities|Time|SetTimerbyEvent (delegate Custom|SetSpeed) 0.5 true))

(fn ConstructionScript)