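; BP_PatrolAiCharacter is a patrol AI character for infiltration mode that feeds perception results into its controller's Blackboard.
; BeginPlay stores the player and its slightly raised starting location.
; AI Perception stimuli write the sound location and re-toggle the hearing key while SeePlayer is false.
; The first PawnSensing sighting, via DoOnce, flags the top-down player as seen, clears hearing, plays an alert sound and shows a timed detection billboard.
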(event OnTargetPerceptionUpdated(AIPerception)
  (params (Actor :type Actor%20Object%20Reference) (Stimulus :type AI%20Stimulus%20Structure))
  (bind _returnvalue (Utilities|Name|MakeLiteralName "hearing?"))
  (bind _self self)
  (bind _returnvalue_2 (AI|GetAIController _self))
  (bind _returnvalue_3 (AI|GetBlackboard _returnvalue_2))
  (if (not (Variables|Default|Get_seePlayer?))
    (AI|Components|Blackboard|SetValueasVector _returnvalue_3 (Utilities|Name|MakeLiteralName "soundLocation") (.StimulusLocation (Utilities|Struct|BreakAIStimulus Stimulus)))
    (AI|Components|Blackboard|SetValueasBool _returnvalue_3 _returnvalue false)
    (AI|Components|Blackboard|SetValueasBool _returnvalue_3 _returnvalue true)))

(event OnSeePawn(PawnSensing)
  (params (Pawn :type Pawn%20Object%20Reference))
  (bind _self self)
  (bind _returnvalue (AI|GetAIController _self))
  (bind _returnvalue_2 (AI|GetBlackboard _returnvalue))
  (Utilities|FlowControl|DoOnce false
    (:Completed
      (Utilities|Casting|CastToBP_TopDownCharacter Pawn)
      (Utilities|FlowControl|Sequence
        (:then_0
          (AI|Components|Blackboard|SetValueasBool _returnvalue_2 (Utilities|Name|MakeLiteralName "seePlayer?") true)
          (AI|Components|Blackboard|SetValueasBool _returnvalue_2 (Utilities|Name|MakeLiteralName "hearing?") false)
          (Audio|PlaySound2D "/Game/CollageAsImpact/Sound/IA_sound/Cue_IA.Cue_IA" 1.0 1.0 0.0 0 0)
          (Utilities|BillBoardFeedBack "/Game/CollageAsImpact/ContentImage/IA/DetectionIa.DetectionIa" 1e+01))))))

(event EventBeginPlay
  (bind _self self)
  (bind _returnvalue (AI|GetAIController _self))
  (bind _returnvalue_2 (AI|GetBlackboard _returnvalue))
  (AI|Components|Blackboard|SetValueasObject _returnvalue_2 (Utilities|Name|MakeLiteralName "player") (Game|GetPlayerCharacter 0))
  (AI|Components|Blackboard|SetValueasVector _returnvalue_2 (Utilities|Name|MakeLiteralName "OgPlace") (+ (Transformation|GetActorLocation) "0.000000,0.000000,10.000000")))

(fn ConstructionScript)