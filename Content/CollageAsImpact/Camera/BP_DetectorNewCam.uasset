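; BP_DetectorNewCam is a camera trigger volume that changes the top-down character's view when it enters the Box.
; Overlap begin targets FirstArm and, with MultiCam enabled, overlap end targets SecondArm; SetNewObjectif caches both arms' transforms and lengths.
; The SwapCam timeline lerps the character's spring arm to the target.
; For the first 80% of the blend, the cursor is reprojected to stay on the world point originally under it.
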(event OnComponentBeginOverlap(Box)
  (params (OverlappedComponent :type Primitive%20Component%20Object%20Reference) (OtherActor :type Actor%20Object%20Reference) (OtherComp :type Primitive%20Component%20Object%20Reference) (OtherBodyIndex :type Integer) (bFromSweep :type Boolean) (SweepResult :type Hit%20Result%20Structure%20%28by%20ref%29))
  (bind _asbp_top_down_character (Utilities|Casting|CastToBP_TopDownCharacter OtherActor))
  (CallFunction|SetNewObjectif (Variables|/Game/TopDown/Blueprints/BP_TopDownCharacter.BP_TopDownCharacter_C|GetSpringArm _asbp_top_down_character) (Variables|Default|GetFirstArm))
  (Variables|Default|SetNeedMousePositionWorld (CallFunction|MouseLocationWorld))
  (bind _percent (Timeline|SwapCam PlayFromStart)
    (:Update
      (Variables|/Script/Engine.SpringArmComponent|SetTargetArmLength (Variables|Objectif|Start|GetStartArm) (Math|Float|Lerp (Variables|Objectif|Start|GetStartLength) (Variables|Objectif|End|GetEndLength) _percent))
      (Transformation|SetRelativeLocationAndRotation (Variables|Objectif|Start|GetStartArm) (Math|Vector|Lerp(Vector) (Variables|Objectif|Start|GetStartLocation) (Variables|Objectif|End|GetEndLocation) _percent) (Math|Rotator|Lerp(Rotator) (Variables|Objectif|Start|GetStartRotation) (Variables|Objectif|End|GetEndRoation) _percent) false false)
      (if (< _percent 0.8)
        (Class|PlayerController|SetMouseLocation (Game|GetPlayerController 0) (Math|Float|Round (.x (.ScreenPosition (Class|GameplayStatics|ProjectWorldtoScreen (Game|GetPlayerController 0) (Variables|Default|GetNeedMousePositionWorld) true)))) (Math|Float|Round (.y (.ScreenPosition (Class|GameplayStatics|ProjectWorldtoScreen (Game|GetPlayerController 0) (Variables|Default|GetNeedMousePositionWorld) true)))))))))

(event OnComponentEndOverlap(Box)
  (params (OverlappedComponent :type Primitive%20Component%20Object%20Reference) (OtherActor :type Actor%20Object%20Reference) (OtherComp :type Primitive%20Component%20Object%20Reference) (OtherBodyIndex :type Integer))
  (if (Variables|Default|GetMultiCam)
    (bind _asbp_top_down_character (Utilities|Casting|CastToBP_TopDownCharacter OtherActor))
    (CallFunction|SetNewObjectif (Variables|/Game/TopDown/Blueprints/BP_TopDownCharacter.BP_TopDownCharacter_C|GetSpringArm _asbp_top_down_character) (Variables|Default|GetSecondArm))
    (Variables|Default|SetNeedMousePositionWorld (CallFunction|MouseLocationWorld))
    (bind _percent (Timeline|SwapCam PlayFromStart)
      (:Update
        (Variables|/Script/Engine.SpringArmComponent|SetTargetArmLength (Variables|Objectif|Start|GetStartArm) (Math|Float|Lerp (Variables|Objectif|Start|GetStartLength) (Variables|Objectif|End|GetEndLength) _percent))
        (Transformation|SetRelativeLocationAndRotation (Variables|Objectif|Start|GetStartArm) (Math|Vector|Lerp(Vector) (Variables|Objectif|Start|GetStartLocation) (Variables|Objectif|End|GetEndLocation) _percent) (Math|Rotator|Lerp(Rotator) (Variables|Objectif|Start|GetStartRotation) (Variables|Objectif|End|GetEndRoation) _percent) false false)
        (if (< _percent 0.8)
          (Class|PlayerController|SetMouseLocation (Game|GetPlayerController 0) (Math|Float|Round (.x (.ScreenPosition (Class|GameplayStatics|ProjectWorldtoScreen (Game|GetPlayerController 0) (Variables|Default|GetNeedMousePositionWorld) true)))) (Math|Float|Round (.y (.ScreenPosition (Class|GameplayStatics|ProjectWorldtoScreen (Game|GetPlayerController 0) (Variables|Default|GetNeedMousePositionWorld) true))))))))))

(event EventBeginPlay)

(event Collision|EventActorBeginOverlap
  (params (OtherActor :type Actor%20Object%20Reference)))

(event EventTick
  (params (DeltaSeconds :type Float%20%28single-precision%29)))

(fn ConstructionScript)

(fn SetNewObjectif
  (params (StartArm :type Spring%20Arm%20Component%20Object%20Reference) (EndArm :type Spring%20Arm%20Component%20Object%20Reference))
  ;[0.15 0.15 0.15 0.5] Start
  (Variables|Objectif|Start|SetStartArm StartArm)
  (Variables|Objectif|Start|SetStartRotation (Variables|/Script/Engine.SceneComponent|GetRelativeRotation StartArm))
  (Variables|Objectif|Start|SetStartLength (Variables|/Script/Engine.SpringArmComponent|GetTargetArmLength StartArm))
  (Variables|Objectif|Start|SetStartLocation (Variables|/Script/Engine.SceneComponent|GetRelativeLocation (Variables|Objectif|Start|GetStartArm)))
  ;[0.15 0.15 0.15 0.5] End
  (Variables|Objectif|End|SetEndArm EndArm)
  (Variables|Objectif|End|SetEndRoation (Variables|/Script/Engine.SceneComponent|GetRelativeRotation EndArm))
  (Variables|Objectif|End|SetEndLength (Variables|/Script/Engine.SpringArmComponent|GetTargetArmLength EndArm))
  (Variables|Objectif|End|SetEndLocation (Variables|/Script/Engine.SceneComponent|GetRelativeLocation (Variables|Objectif|End|GetEndArm)))
  (return))

(fn MouseLocationWorld
  (return (.Location (Collision|BreakHitResult (.HitResult (Game|Player|GetHitResultUnderCursorbyChannel (Game|GetPlayerController 0) "TraceTypeQuery1" true))))))