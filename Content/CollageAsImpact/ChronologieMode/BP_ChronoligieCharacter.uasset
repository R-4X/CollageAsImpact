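; Player character for the Chronologie mode, where the mouse drags picture objects between places to reorder them.
; Enhanced Input drives a cursor trace that picks up a BP_ObjectChronologie and keeps it hovering above the traced surface.
; All pictures lose collision during a drag so traces pass through them.
; On release, a downward trace swaps the picture with the occupant of the BP_Place below, or returns it to its current place.
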(event Input|EnhancedActionEvents|EnhancedInputActionIA_DragAndDrop
  (params (ActionValue :type Boolean) (ElapsedSeconds :type Float%20%28double-precision%29) (TriggeredSeconds :type Float%20%28double-precision%29) (InputAction :type Input%20Action%20Object%20Reference :default "/Game/CollageAsImpact/ChronologieMode/Control/Action/IA_DragAndDrop.IA_DragAndDrop"))
  (:Triggered
    (CallFunction|Drag))
  (:Started
    (CallFunction|TakeObject))
  (:Canceled
    (CallFunction|StopDrag :!label _label)
    (Audio|PlaySound2D "/Engine/EditorSounds/GamePreview/PossessPlayer.PossessPlayer" 1.0 1.0 0.0 0 0))
  (:Completed
    (goto _label)))

(event EventBeginPlay
  (bind _outactors (Actor|GetAllActorsOfClass "/Game/CollageAsImpact/ChronologieMode/Photo/TakePicture/Object/BP_ObjectChronologie.BP_ObjectChronologie_C"))
  (Variables|Default|Set_pictures _outactors))

(fn ConstructionScript)

(fn TakeObject
  (bind (_location _direction) (CallFunction|GetMouseLocation))
  (bind _outhit (Collision|LineTraceByChannel _location _direction "TraceTypeQuery1" false 0 "None"))
  (bind _output_get (LocalVariables|SetHitActor (.HitActor (Collision|BreakHitResult _outhit))))
  (bind _asbp_object_chronologie (Utilities|Casting|CastToBP_ObjectChronologie _output_get))
  (Variables|Default|Set_whatITake _asbp_object_chronologie)
  (CallFunction|EnableCollisionPictures false)
  (return))

(fn GetMouseLocation
  (bind _returnvalue (Game|GetPlayerController 0))
  (bind (_worldlocation _worlddirection) (Game|Player|ConvertMouseLocationToWorldSpace _returnvalue))
  (return _worldlocation (+ _worlddirection (* _worlddirection (Variables|Default|Get_range)))))

(fn Drag
  (bind (_location _direction) (CallFunction|GetMouseLocation))
  (Utilities|IsValid (Variables|Default|Get_whatITake)
    (:Is%20Valid
      (bind _outhit (Collision|LineTraceByChannel _location _direction "TraceTypeQuery1" false 0 "None"))
      (Transformation|SetActorLocation (Variables|Default|Get_whatITake) (Math|Vector|MakeVector (.X (Math|Vector|BreakVector (.Location (Collision|BreakHitResult _outhit)))) (.Y (Math|Vector|BreakVector (.Location (Collision|BreakHitResult _outhit)))) (+ (.Z (Math|Vector|BreakVector (.Location (Collision|BreakHitResult _outhit)))) 1e+02)) false false))))

(fn StopDrag
  (Utilities|IsValid (Variables|Default|Get_whatITake)
    (:Is%20Valid
      (bind (_outhit _returnvalue) (Collision|LineTraceByChannel (Transformation|GetActorLocation (Variables|Default|Get_whatITake)) (+ (Transformation|GetActorLocation (Variables|Default|Get_whatITake)) (* (Transformation|GetActorUpVector (Variables|Default|Get_whatITake)) (LocalVariables|Get_rangeDown) -1.0)) "TraceTypeQuery1" false 0 "None"))
      (if _returnvalue
        (bind _asbp_place (Utilities|Casting|CastToBP_Place (.HitActor (Collision|BreakHitResult _outhit)))
          (:then
            (CallFunction|SwapPicture _asbp_place)
            (CallFunction|EnableCollisionPictures true)
            (Variables|Default|Set_whatITake 0))
          (:CastFailed
            (Transformation|SetActorLocation (Variables|Default|Get_whatITake) (Transformation|GetActorLocation (Variables|/Game/CollageAsImpact/ChronologieMode/Photo/TakePicture/Object/BP_ObjectChronologie.BP_ObjectChronologie_C|Get_currentPlace (Variables|Default|Get_whatITake))) false false :!label _label)
            (CallFunction|EnableCollisionPictures true)
            (Variables|Default|Set_whatITake 0)))
        (else
          (goto _label))))))

(fn EnableCollisionPictures
  (params (bNewActorEnableCollision :type Boolean))
  (for _array_element (Variables|Default|Get_pictures)
    (Collision|SetActorEnableCollision _array_element bNewActorEnableCollision))
  (return))

(fn SwapPicture
  (params (NewPlace :type BP%20Place%20Object%20Reference))
  (bind __currentpicture (Variables|/Game/CollageAsImpact/ChronologieMode/Photo/TakePicture/Place/BP_Place.BP_Place_C|Get_currentPicture NewPlace))
  (bind __whatitake (Variables|Default|Get_whatITake))
  (bind _output_get (LocalVariables|SetCurrentPlaceOld (Variables|/Game/CollageAsImpact/ChronologieMode/Photo/TakePicture/Object/BP_ObjectChronologie.BP_ObjectChronologie_C|Get_currentPlace __currentpicture)))
  (Variables|/Game/CollageAsImpact/ChronologieMode/Photo/TakePicture/Object/BP_ObjectChronologie.BP_ObjectChronologie_C|Set_currentPlace __currentpicture (Variables|/Game/CollageAsImpact/ChronologieMode/Photo/TakePicture/Object/BP_ObjectChronologie.BP_ObjectChronologie_C|Get_currentPlace __whatitake))
  (Variables|/Game/CollageAsImpact/ChronologieMode/Photo/TakePicture/Object/BP_ObjectChronologie.BP_ObjectChronologie_C|Set_currentPlace __whatitake _output_get)
  (Default|PutDown __currentpicture)
  (Default|PutDown __whatitake))