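; BP_Door is a locked door that swings open 90 degrees in yaw once its key has been picked up.
; Interact and a player character overlapping Box1 share the same logic, gated by HasKey, which PickUpKey sets.
; Each attempt adds a new WBP_BackGround widget to the viewport and also requires that widget's HaveKey flag.
; A FlipFlop then alternately plays and reverses a Timeline that rotates the root component.
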(event OnComponentBeginOverlap(Box1)
  (params (OverlappedComponent :type Primitive%20Component%20Object%20Reference) (OtherActor :type Actor%20Object%20Reference) (OtherComp :type Primitive%20Component%20Object%20Reference) (OtherBodyIndex :type Integer) (bFromSweep :type Boolean) (SweepResult :type Hit%20Result%20Structure%20%28by%20ref%29))
  (Utilities|Casting|CastToBP_TopDownCharacter OtherActor)
  (if (Variables|Default|GetHasKey?)
    (bind _returnvalue (UserInterface|CreateWidget "/Game/CollageAsImpact/Door/Widget/WBP_BackGround.WBP_BackGround_C"))
    (UserInterface|Viewport|AddtoViewport _returnvalue 0)
    (if (Variables|/Game/CollageAsImpact/Door/Widget/WBP_BackGround.WBP_BackGround_C|GetHave%20Key _returnvalue)
      (Utilities|FlowControl|FlipFlop
        (:A
          (bind _open (Timeline|Timeline Play)
            (:Update
              (Transformation|SetRelativeRotation (Variables|Default|GetDefaultSceneRoot) (Math|Rotator|MakeRotator 0.0 0.0 (Math|Float|Lerp 0.0 9e+01 _open)) false false))))
        (:B
          (Timeline|Timeline Reverse))))))

(event EventPickUpKey
  (Variables|Default|SetHasKey? true))

(event EventInteract
  (if (Variables|Default|GetHasKey?)
    (bind _returnvalue (UserInterface|CreateWidget "/Game/CollageAsImpact/Door/Widget/WBP_BackGround.WBP_BackGround_C"))
    (UserInterface|Viewport|AddtoViewport _returnvalue 0)
    (if (Variables|/Game/CollageAsImpact/Door/Widget/WBP_BackGround.WBP_BackGround_C|GetHave%20Key _returnvalue)
      (Utilities|FlowControl|FlipFlop
        (:A
          (bind _open (Timeline|Timeline Play)
            (:Update
              (Transformation|SetRelativeRotation (Variables|Default|GetDefaultSceneRoot) (Math|Rotator|MakeRotator 0.0 0.0 (Math|Float|Lerp 0.0 9e+01 _open)) false false))))
        (:B
          (Timeline|Timeline Reverse))))))

(fn ConstructionScript)