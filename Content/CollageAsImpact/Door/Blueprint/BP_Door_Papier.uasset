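; BP_Door_Papier is a door actor that serves as a transition to the MAP_Dialogue level.
; OpenDoor uses a FlipFlop to alternately play and reverse a timeline.
; Timeline updates reapply the root's current relative rotation, with no track value visibly driving it.
; When the timeline finishes, it activates a Niagara effect, then opens the level after a short delay.
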(event EventBeginPlay)

(event Collision|EventActorBeginOverlap
  (params (OtherActor :type Actor%20Object%20Reference)))

(event EventTick
  (params (DeltaSeconds :type Float%20%28single-precision%29)))

(event EventOpenDoor
  (bind _defaultsceneroot (Variables|Default|GetDefaultSceneRoot))
  (bind _relativerotation (Variables|/Script/Engine.SceneComponent|GetRelativeRotation _defaultsceneroot))
  (Utilities|FlowControl|FlipFlop
    (:A
      (Timeline|Timeline_0 Play
        (:Update
          (Transformation|SetRelativeRotation _defaultsceneroot (Math|Rotator|MakeRotator (.roll _relativerotation) (.pitch _relativerotation) (.yaw _relativerotation)) false false))
        (:Finished
          (Components|Activation|Activate (Variables|Default|GetNiagara) true)
          (Utilities|FlowControl|Delay 2.0)
          (Game|OpenLevel(byObjectReference) "/Game/CollageAsImpact/Level/MAP_Dialogue.MAP_Dialogue"))))
    (:B
      (Timeline|Timeline_0 Reverse))))

(fn ConstructionScript
  (|CallParentFunction))